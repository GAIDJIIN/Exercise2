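; BP_Spawner is a nest that spawns a deer and sends it toward TargetToMove.
; The DeerToSpawn enum picks one of three AI controller classes and numbers the nest's label in the construction script.
; SpawnDeer creates the deer and controller, possesses, starts movement and plays a sound, or prints an error without a target.
; The deer's destruction is bound to an event, with OnDestroyedDeer calling CanSpawnDeer.
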(fn ConstructionScript
  (Rendering|Components|TextRender|SetText (Variables|Default|GetSpawnerName) (Utilities|Text|FormatText "Гнездо-{Num}" (Utilities|String|ToString(Byte) (+ (Variables|SpawnInfo|GetDeerToSpawn) 1)))))

(fn SpawnDeer
  (Variables|SpawnInfo|GetTargetToMove
    (:then
      (bind _returnvalue (Game|SpawnActorfromClass "/Game/Blueprints/Deer/BP_Deer.BP_Deer_C" (Math|Transform|MakeTransform (Transformation|GetActorLocation) (Transformation|GetWorldRotation (Variables|Default|GetSpawnRotation))) "Undefined" self 0))
      (LocalVariables|SetLocalDeer _returnvalue)
      (bind _output_get (LocalVariables|SetLocalAIController (Utilities|Select :Index (Variables|SpawnInfo|GetDeerToSpawn) :NewEnumerator0 "/Game/Blueprints/Deer/BP_DeerAIController1.BP_DeerAIController1_C" :NewEnumerator1 "/Game/Blueprints/Deer/AIControllers/BP_DeerAIController2.BP_DeerAIController2_C" :NewEnumerator2 "/Game/Blueprints/Deer/AIControllers/BP_DeerAIController3.BP_DeerAIController3_C")))
      (bind _returnvalue_2 (Game|SpawnActorfromClass _output_get (Math|Transform|MakeTransform "0, 0, 0") "Undefined" (LocalVariables|GetLocalDeer) (Variables|SpawnInfo|GetTargetToMove) self (LocalVariables|GetLocalDeer)))
      (Pawn|Possess _returnvalue_2 (LocalVariables|GetLocalDeer))
      (Default|StartMoving _returnvalue_2)
      (Game|BindEventtoOnDestroyed (LocalVariables|GetLocalDeer) (EventDispatchers|CreateEvent :!event OnDestroyedDeer))
      (Audio|PlaySoundatLocation "/Game/Sounds/DeerSound/Spawn.Spawn" (Transformation|GetActorLocation) "0, 0, 0" 1.0 1.0 0.0 0 0 0)
      (return))
    (:else
      (Development|PrintString "ВЫБЕРИТЕ ПУНКТ НАЗНАЧЕНИЯ!!!! 
(Target To Move)" true true "(R=1.000000,G=0.000000,B=0.008526,A=1.000000)" 5.0))))

(fn OnDestroyedDeer
  (params (Destroyed%20Actor :type Actor%20Object%20Reference))
  (Default|CallCanSpawnDeer))