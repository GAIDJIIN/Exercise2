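; BP_Button is an interactable button that tells its linked Spawner to spawn a deer.
; A press locks the button, zeroes the mesh's "Enable" material parameter and plays a sound.
; BeginPlay binds to the Spawner's CanSpawnDeer dispatcher to allow pressing again once the deer reaches its point and disappears.
; The construction script labels the button with the Spawner's name, and a missing Spawner triggers red on-screen warnings at runtime.
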(event EventBeginPlay
  ;[1 1 1] Биндим ивент для того, чтобы мы смогли снова нажимать кнопку, после того как олень дойдет до точки и исчезнет
  (bind _spawner (Variables|Spawner|GetSpawner)
    (:then
      (EventDispatchers|AssignCanSpawnDeer _spawner (EventDispatchers|CreateEvent :!event CanPressAgain)))
    (:else
      (Development|PrintString "ВЫБЕРИТЕ ТОЧКУ СПАВНА!!! 
(Spawner)" true true "(R=1.000000,G=0.003835,B=0.000000,A=1.000000)" 5.0))))

(event EventInteractLogic
  (if (Variables|Status|GetbCanPress)
    (bind _spawner (Variables|Spawner|GetSpawner)
      (:then
        (Default|SpawnDeer _spawner)
        (Variables|Status|SetbCanPress false)
        (Rendering|Material|SetScalarParameterValueonMaterials (Variables|Default|GetButtonMesh) "Enable" 0.0)
        (Audio|PlaySoundatLocation "/Game/Sounds/Button_Pressed.Button_Pressed" (Transformation|GetActorLocation) "0, 0, 0" 1.0 1.0 0.0 0 0 0))
      (:else
        (Development|PrintString "ВЫБЕРИТЕ ТОЧКУ СПАВНА!!! 
(Spawner)" true true "(R=1.000000,G=0.003835,B=0.000000,A=1.000000)" 5.0)))))

(fn ConstructionScript
  ;[1 1 1] Отображение имени гнезда, к которому привязана
  (bind _spawner (Variables|Spawner|GetSpawner)
    (:then
      (Rendering|Components|TextRender|SetText (Variables|Default|GetButtonName) (Utilities|Text|FormatText "Кнопка 
({SpawnerName})" (Variables|/Script/Engine.TextRenderComponent|GetText (Variables|/Game/Blueprints/Gnezdo/BP_Spawner.BP_Spawner_C|GetSpawnerName _spawner)))))
    (:else)))

(fn CanPressAgain
  (Variables|Status|SetbCanPress true)
  (Rendering|Material|SetScalarParameterValueonMaterials (Variables|Default|GetButtonMesh) "Enable" 3.0))