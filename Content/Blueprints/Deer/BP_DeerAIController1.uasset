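; AI controller for the deer that sends it to a target actor and removes it on arrival.
; On possession it caches the BP_Deer pawn, and StartMoving passes the stored TargetToMove to GoToLocation, which runs AI MoveTo.
; When the move succeeds, it hides the deer, plays the Destroy sound at its location and gives it a short lifespan.
; Getters expose the spawner and both target references.
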(event Custom|GoToLocation
  (params (TargetToMove :type Actor%20Object%20Reference))
  (bind _returnvalue (Pawn|GetControlledPawn))
  (Utilities|IsValid TargetToMove
    (:Is%20Valid
      (Variables|InfoforMoving|SetCurrentTarget TargetToMove)
      (Utilities|IsValid _returnvalue
        (:Is%20Valid
          (AI|AIMoveTo _returnvalue "0, 0, 0" (Variables|InfoforMoving|GetCurrentTarget) 1e+01 false
            (:OnSuccess
              (ServiceLogic|OnSuccessLogic))))))))

(event EventPossess
  (params (PossessedPawn :type Pawn%20Object%20Reference))
  (bind _asbp_deer (Utilities|Casting|CastToBP_Deer PossessedPawn))
  (Variables|Default|SetDeerPawn _asbp_deer))

(fn ConstructionScript)

(fn GetCurrentTarget
  (return (Variables|InfoforMoving|GetCurrentTarget)))

(fn StartMovingLogic
  (CallFunction|GotoLocation (Variables|InfoForMoving|GetTargetToMove)))

(fn StartMoving
  (bind _targettomove (Variables|InfoForMoving|GetTargetToMove)
    (:then
      (Variables|InfoforMoving|SetCurrentTarget _targettomove)
      (ServiceLogic|StartMovingLogic))
    (:else)))

(fn OnSuccessLogic
  (bind _deerpawn (Variables|Default|GetDeerPawn)
    (:then
      (Default|Hide _deerpawn)
      (Audio|PlaySoundatLocation "/Game/Sounds/DeerSound/Destroy.Destroy" (Transformation|GetActorLocation (Pawn|GetControlledPawn)) "0, 0, 0" 1.0 1.0 0.0 0 0 0)
      (Actor|SetLifeSpan (Pawn|GetControlledPawn) 2.0))
    (:else)))

(fn GetSpawner
  (return (Variables|InfoforMoving|GetSpawner)))

(fn GetTargettoMove
  (return (Variables|InfoForMoving|GetTargetToMove)))