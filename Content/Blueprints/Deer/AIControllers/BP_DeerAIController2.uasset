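; Deer AI controller variant that moves toward a target and can pause movement on timed intervals.
; StartMovingLogic calls StartMove, which sets a MoveTime timer and sends the deer to the location from GetTargetToMove.
; StopMove halts movement and sets a WaitTime timer, reusing the same timer handle.
; On success, it runs the parent logic and clears that timer.
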(fn ConstructionScript
  (|CallParentFunction))

(fn StopMove
  (AI|Navigation|StopMovement)
  (bind _returnvalue (Utilities|Time|SetTimerbyEvent (EventDispatchers|CreateEvent :!event StartMove) (Variables|Timer|GetWaitTime)))
  (Variables|Timer|SetMoveTimerHandle _returnvalue))

(fn StartMove
  (bind _returnvalue (Utilities|Time|SetTimerbyEvent (EventDispatchers|CreateEvent :!event StopMove) (Variables|Timer|GetMoveTime)))
  (Variables|Timer|SetMoveTimerHandle _returnvalue)
  (CallFunction|GotoLocation (CallFunction|GetTargettoMove)))

(fn StartMovingLogic
  (MoveLogic|StartMove))

(fn OnSuccessLogic
  (|CallParentFunction)
  (Utilities|Time|ClearandInvalidateTimerbyHandle (Variables|Timer|GetMoveTimerHandle)))